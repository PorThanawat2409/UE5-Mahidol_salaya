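; Modular toon teen boy pawn (variant B) whose outfit can be randomized in the construction script.
; Clothing, hood and glasses meshes follow the main Mesh as leader pose component, sharing its animation.
; When the Randomize flag is set, Randomizer rolls glasses, jacket and hood state, then clears the flag.
; It always applies the stored booleans as visibility, showing exactly one of the two hood meshes.
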(fn `UserConstructionScript`
  (bind _hoodupdown (`self.HoodUpDown`))
  (`SkinnedMeshComponent.SetLeaderPoseComponent` (`self.TTSweater`) (`self.Mesh`) false false)
  (`SkinnedMeshComponent.SetLeaderPoseComponent` (`self.TTJacket`) (`self.Mesh`) false false)
  (`SkinnedMeshComponent.SetLeaderPoseComponent` (`self.TTFeetB`) (`self.Mesh`) false false)
  (`SkinnedMeshComponent.SetLeaderPoseComponent` (`self.TTLegsLD`) (`self.Mesh`) false false)
  (`SkinnedMeshComponent.SetLeaderPoseComponent` (`self.TTHoodA`) (`self.Mesh`) false false)
  (`SkinnedMeshComponent.SetLeaderPoseComponent` (`self.TTHoodB`) (`self.Mesh`) false false)
  (`SkinnedMeshComponent.SetLeaderPoseComponent` (`self.TTGlasses`) (`self.Mesh`) false false)
  (if (`self.Randomize`)
    (set `self.Glasses` (`KismetMathLibrary.RandomBool`))
    (set `self.JacketON` (`KismetMathLibrary.RandomBool`))
    (set `self.HoodUpDown` (`KismetMathLibrary.RandomBool`))
    (set `self.Randomize` (not true)))
  (`SceneComponent.SetVisibility` (`self.TTGlasses`) (`self.Glasses`) false)
  (`SceneComponent.SetVisibility` (`self.TTHoodA`) _hoodupdown false)
  (`SceneComponent.SetVisibility` (`self.TTHoodB`) (not _hoodupdown) false)
  (`SceneComponent.SetVisibility` (`self.TTJacket`) (`self.JacketON`) false))